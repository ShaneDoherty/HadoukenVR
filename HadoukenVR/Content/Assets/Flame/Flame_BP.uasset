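; Flame actor for VR that scales and dims with the distance between the player's two motion controllers.
; Tick measures the hand gap and maps it through clamped ranges to actor scale and point light intensity, so the flame fades as hands separate.
; A timeline flicker curve modulates the light.
; A looping timer runs FaceFlame to yaw the actor toward the camera, billboard-style, on the horizontal plane.
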(event EventTick
  (params (DeltaSeconds :type Float%20%28single-precision%29))
  (bind _returnvalue (Game|Player|GetPlayerPawn 0))
  (bind _asmotion_controller_pawn (Utilities|Casting|CastToMotionControllerPawn _returnvalue))
  (bind _asmotion_controller_pawn_2 (Utilities|Casting|CastToMotionControllerPawn _returnvalue))
  (bind _output_get (Variables|Default|SetHandDistance (Math|Vector|VectorLength (- (Transformation|GetWorldLocation (Variables|/Game/VirtualRealityBP/Blueprints/BP_MotionController.BP_MotionController_C|GetMotionController (Variables|/Game/VirtualRealityBP/Blueprints/MotionControllerPawn.MotionControllerPawn_C|GetLeftController _asmotion_controller_pawn))) (Transformation|GetWorldLocation (Variables|/Game/VirtualRealityBP/Blueprints/BP_MotionController.BP_MotionController_C|GetMotionController (Variables|/Game/VirtualRealityBP/Blueprints/MotionControllerPawn.MotionControllerPawn_C|GetRightController _asmotion_controller_pawn_2)))))))
  (Transformation|SetActorScale3D (Math|Vector|MakeVector (Math|Float|MapRangeClamped _output_get 0.0 2e+01 1.0 0.0) (Math|Float|MapRangeClamped _output_get 0.0 2e+01 1.0 0.0) (Math|Float|MapRangeClamped _output_get 0.0 2e+01 1.0 0.0)))
  (bind _flicker (Timeline|Timeline_0 Play)
    (:Update
      (Rendering|Components|Light|SetIntensity (Variables|Default|GetPointLight) (* (Math|Float|MapRangeClamped (Variables|Default|GetHandDistance) 0.0 2e+01 2.0 -1.0) _flicker)))))

(event Collision|EventActorBeginOverlap
  (params (OtherActor :type Actor%20Object%20Reference)))

(event EventBeginPlay
  (Utilities|Time|SetTimerbyFunctionName 0 "FaceFlame" 0.1 true))

(fn ConstructionScript)

(fn FaceFlame
  (Transformation|SetActorRotation (Math|Conversions|RotationFromXVector (Math|Vector|Normalize (* (- (Camera|GetCameraLocation (Game|GetPlayerCameraManager 0)) (Transformation|GetActorLocation)) "1.000000,1.000000,0.000000")))))