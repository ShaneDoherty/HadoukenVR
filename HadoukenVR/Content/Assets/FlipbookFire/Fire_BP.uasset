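; Fire_BP is a fire actor that turns to face the player camera like a billboard.
; On BeginPlay it starts a looping timer that calls GetAngle ten times a second instead of using Tick.
; GetAngle flattens the direction to the camera onto the horizontal plane, so the actor only yaws.
; A light flicker timeline and point light intensity update are present but never run.
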(event EventBeginPlay
  (Utilities|Time|SetTimerbyFunctionName 0 "GetAngle" 0.1 true))

(event Collision|EventActorBeginOverlap
  (params (OtherActor :type Actor%20Object%20Reference)))

(event EventTick
  (params (DeltaSeconds :type Float%20%28single-precision%29)))

(fn ConstructionScript)

(fn GetAngle
  (Transformation|SetActorRotation (Math|Conversions|RotationFromXVector (Math|Vector|Normalize (* (- (Camera|GetCameraLocation (Game|GetPlayerCameraManager 0)) (Transformation|GetActorLocation)) "1.000000,1.000000,0.000000")))))